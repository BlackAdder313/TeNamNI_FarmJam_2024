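; BP_Wheat is a wheat plant actor that visually grows by scaling up its root component in two stages.
; From a small construction scale, Tick calls GrowSprout, which applies GrowWheatByRandomNumber's scale until it passes the sprout target, then clamps it and disables tick.
; OnWheatCollectionStart extends the parent event, raises the target to full size and re-enables tick after a random delay, staggering growth between plants.
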(event EventBeginPlay
  (Variables|Default|SetGrowFullWheat false))

(event Collision|EventActorBeginOverlap
  (params (OtherActor :type Actor%20Object%20Reference)))

(event EventTick
  (params (DeltaSeconds :type Float%20%28single-precision%29))
  (if (Variables|Default|GetGrowFullWheat)
    (CallFunction|GrowSprout 1.3)
    (else
      (CallFunction|GrowSprout 0.65))))

(event EventOnWheatCollectionStart
  (|CallParentFunction)
  (Variables|Default|SetGrowFullWheat true)
  (Utilities|FlowControl|Delay (Math|Random|RandomFloatinRange 0.5 4.5))
  (Actor|Tick|SetActorTickEnabled true))

(fn ConstructionScript
  (Transformation|SetWorldScale3D (Variables|Default|GetDefaultSceneRoot) "0.350000,0.350000,0.350000"))

(fn GrowSprout
  (params (target :type Float%20%28double-precision%29))
  (bind _returnvalue (|GrowWheatByRandomNumber))
  (if (> (Class|KismetMathLibrary|GetMinElement _returnvalue) target)
    (Transformation|SetWorldScale3D (Variables|Default|GetDefaultSceneRoot) (Math|Conversions|ToVector(Float) target))
    (Actor|Tick|SetActorTickEnabled false)
    (else
      (Transformation|SetWorldScale3D (Variables|Default|GetDefaultSceneRoot) _returnvalue))))
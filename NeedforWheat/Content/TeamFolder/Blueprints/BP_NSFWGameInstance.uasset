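; BP_NSFWGameInstance is a game instance that keeps a high score for each level in the HighScores map, keyed by level name.
; The UpdateHighScore event stores the higher of the saved and submitted scores, or adds the submitted score for a new level.
; GetHighScore returns the saved value for a level; its fallback that would add and return zero for a missing level is unconnected.
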(event Custom|UpdateHighScore
  (params (LevelName :type String) (Score :type Integer))
  (bind _highscores (Variables|Default|GetHighScores))
  (bind (_value _returnvalue) (Utilities|Map|Find _highscores LevelName))
  (if _returnvalue
    (Utilities|Map|Add (Variables|Default|GetHighScores) LevelName (Math|Integer|Max(Integer) _value Score))
    (else
      (Utilities|Map|Add (Variables|Default|GetHighScores) LevelName Score))))

(fn GetHighScore
  (params (LevelName :type String))
  (bind _highscores (Variables|Default|GetHighScores))
  (bind (_value _returnvalue) (Utilities|Map|Find _highscores LevelName))
  (if _returnvalue
    (return _value)))